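; BP_FMPlayerController is a player controller that gives the player a toggleable character change widget.
; On BeginPlay it creates UI_CharacterChange_Actual, stores it as DressChangeWidgetRef, adds it to the viewport and collapses it.
; The Tab key drives a FlipFlop that alternates the widget between visible and collapsed.
; Both branches turn the mouse cursor on, so it stays shown after the widget closes.
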(event `self.ReceiveBeginPlay`
  (bind _returnvalue (`|CreateWidget` "/Game/Widget/UI_CharacterChange_Actual.UI_CharacterChange_Actual_C" (`GameplayStatics.GetPlayerController` 0)))
  (bind _output_get (set `self.DressChangeWidgetRef` _returnvalue))
  (`UserWidget.AddToViewport` _output_get 0)
  (`Widget.SetVisibility` _output_get "Collapsed"))

(event `Key|Tab`
  (params (Key :type "Key Structure"))
  (bind _dresschangewidgetref (`self.DressChangeWidgetRef`))
  ;[1 1 1] Showing the Change Widget
  (:`Pressed`
    (`/Engine/EditorBlueprintResources/StandardMacros.FlipFlop`
      (:`A`
        (`Widget.SetVisibility` _dresschangewidgetref "Visible")
        (set `self.bShowMouseCursor` true))
      (:`B`
        (`Widget.SetVisibility` _dresschangewidgetref "Collapsed")
        (set `self.bShowMouseCursor` true)))))

(fn `UserConstructionScript`)